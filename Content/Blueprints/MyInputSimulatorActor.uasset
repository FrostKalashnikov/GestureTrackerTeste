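; Debug actor for testing arrow direction detection and key input, with disconnected input-simulation logic.
; Each Tick prints the forward dot product of two arrows, then labels the target Up, Right or Left relative to the source using dot products and a threshold.
; Any key press or release prints the key name in a distinct color.
; Unwired chains would replay a test key sequence as timed simulated presses and releases; BeginPlay only runs a delay.
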(event `self.ReceiveBeginPlay`
  (`KismetSystemLibrary.Delay` 2.0))

(event `Key|AnyKey`
  (params (Key :type "Key Structure"))
  (bind _returnvalue (`self.ConvertKeyToString` Key))
  (:`Pressed`
    (`KismetSystemLibrary.PrintString` _returnvalue true true (struct :`R` 1.0 :`G` 0.176995 :`A` 1.0)))
  (:`Released`
    (`KismetSystemLibrary.PrintString` _returnvalue true true (struct :`R` 0.083333 :`B` 1.0 :`A` 1.0))))

(event `self.ReceiveTick`
  (params (DeltaSeconds :type "Float (single-precision)"))
  (bind _returnvalue (`SceneComponent.K2_GetComponentRotation` (`self.ArrowSource`)))
  (bind _returnvalue_2 (`KismetMathLibrary.GetForwardVector` (`SceneComponent.K2_GetComponentRotation` (`self.ArrowTarget`))))
  (bind _returnvalue_3 (`KismetMathLibrary.Dot_VectorVector` _returnvalue_2 (`KismetMathLibrary.GetRightVector` _returnvalue)))
  (`KismetSystemLibrary.PrintString` (`KismetStringLibrary.Conv_DoubleToString` (`KismetMathLibrary.Dot_VectorVector` (`KismetMathLibrary.GetForwardVector` _returnvalue) _returnvalue_2)) true true (struct :`G` 0.66 :`B` 1.0 :`A` 1.0) 2.0 "Dir")
  (if (> (`KismetMathLibrary.Dot_VectorVector` _returnvalue_2 (`KismetMathLibrary.GetUpVector` _returnvalue)) 0.9)
    (`KismetSystemLibrary.PrintString` "Up" true true (struct :`R` 1.0 :`G` 0.345901 :`A` 1.0) 2.0 "Arrow") ; To UP
    (elif (> _returnvalue_3 0.9)
      (`KismetSystemLibrary.PrintString` "Right" true true (struct :`R` 1.0 :`G` 0.345901 :`A` 1.0) 2.0 "Arrow") ; To Right
      (elif (< _returnvalue_3 -0.9)
        (`KismetSystemLibrary.PrintString` "Left" true true (struct :`R` 1.0 :`G` 0.345901 :`A` 1.0) 2.0 "Arrow") ; To Left
      ))))

(fn `ConvertKeyToString`
  (params (Key :type "Key Structure (by ref)"))
  (returns (ReturnValue :type String))
  (return (`KismetTextLibrary.Conv_TextToString` (`KismetInputLibrary.Key_GetDisplayName` Key))))

(fn `UserConstructionScript`)